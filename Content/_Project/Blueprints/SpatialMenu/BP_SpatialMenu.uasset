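; BP_SpatialMenu is a spatial menu that shows a gaze cursor where the player's gaze interaction ray hits it.
; On BeginPlay it caches the player pawn's WidgetInteractionComponent tagged "GazeInteraction".
; Each Tick it reads that component's last hit result and moves GazeCursor to the impact point.
; The cursor shows only when the hit actor casts to BP_SpatialMenu, so any instance qualifies, and hides otherwise.
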(event EventBeginPlay
  (CallFunction|GetWidgetInteraction))

(event EventTick
  (params (DeltaSeconds :type Float%20%28single-precision%29))
  (CallFunction|SetRayPosition))

(fn ConstructionScript)

(fn GetWidgetInteraction
  (for _array_element (Actor|GetComponentsbyTag (Game|Player|GetPlayerPawn 0) "/Script/UMG.WidgetInteractionComponent" "GazeInteraction")
    (Variables|Default|SetgazeInteractionRef _array_element)))

(fn SetRayPosition
  (bind _gazeinteractionref (Variables|Default|GetgazeInteractionRef))
  (bind _returnvalue (Class|WidgetInteractionComponent|GetLastHitResult _gazeinteractionref))
  (bind (_bblockinghit _binitialoverlap _time _distance _location _impactpoint _normal _impactnormal _physmat _hitactor) (Collision|BreakHitResult _returnvalue))
  (Variables|Default|SethitLocation _impactpoint)
  (Utilities|Casting|CastToBP_SpatialMenu _hitactor
    (:then
      (Transformation|SetWorldLocation (Variables|Default|GetGazeCursor) (Variables|Default|GethitLocation) false false)
      (Rendering|SetVisibility (Variables|Default|GetGazeCursor) true false))
    (:CastFailed
      (Rendering|SetVisibility (Variables|Default|GetGazeCursor) false false))))